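; Harmful crystal pickup actor that, on any sphere overlap, flies into the player and deals damage.
; It caches its location, scale and light intensity, then a timeline lerps it toward player pawn 0 while shrinking it to zero.
; LightFlickering sets the point light straight to zero, leaving its intensity lerp unused.
; When the timeline finishes, it damages the overlapping actor, which is not filtered to the player, and destroys itself.
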(event `self.Sphere.OnComponentBeginOverlap`
  (params (OverlappedComponent :type "PrimitiveComponent Object Reference") (OtherActor :type "Actor Object Reference") (OtherComp :type "PrimitiveComponent Object Reference") (OtherBodyIndex :type Integer) (bFromSweep :type Boolean) (SweepResult :type "HitResult Structure (by ref)"))
  (`self.Set Properties`)
  (bind (_direction _smooth_lerp_alpha _lerp_scale _lerp_light) (`Timeline|Timeline_0`)
    (:`Update`
      (`self.animation_movement` _smooth_lerp_alpha)
      (`self.Animation Scale` _lerp_scale)
      (`self.Light Flickering` _lerp_light))
    (:`Finished`
      (`self.Damage&destroy` OtherActor))))

(fn `Animation Scale`
  (params (Alpha :type "Float (double-precision)"))
  (`self.SetActorScale3D` (`KismetMathLibrary.VLerp` (`self.crystal_scale`) (0.0 0.0 0.0) Alpha)))

(fn `animation_movement`
  (params (Alpha :type "Float (double-precision)"))
  (`self.K2_SetActorLocation` (`KismetMathLibrary.VLerp` (`self.crystal_location`) (`self.K2_GetActorLocation` (`GameplayStatics.GetPlayerPawn` 0)) Alpha)))

(fn `Damage&destroy`
  (params (DamagedActor :type "Actor Object Reference"))
  (`GameplayStatics.ApplyDamage` DamagedActor 1.0)
  (`self.K2_DestroyActor`))

(fn `Light Flickering`
  (params (Alpha :type "Float (double-precision)"))
  (`LightComponent.SetIntensity` (`self.PointLight`) 0.0))

(fn `Set Properties`
  (set `self.crystal_location` (`self.K2_GetActorLocation`))
  (set `self.crystal_scale` (`self.GetActorScale3D`))
  (set `self.crystal_intensity` (`LightComponentBase.Intensity` (`self.PointLight`))))

(fn `UserConstructionScript`)