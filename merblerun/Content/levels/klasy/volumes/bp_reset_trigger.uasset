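; Level reset trigger volume that restarts the current level when the first player's pawn overlaps its box.
; On BeginPlay, a Fade graph fades the camera in from fully faded.
; The overlap applies damage, then the Fade&restart graph fades the camera out and reopens the level by name after a short delay.
; Tick refreshes the cached current level name every frame for that reload.
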(event `self.ReceiveBeginPlay`
  (`self.Fade`))

(event `self.Box.OnComponentBeginOverlap`
  (params (OverlappedComponent :type "PrimitiveComponent Object Reference") (OtherActor :type "Actor Object Reference") (OtherComp :type "PrimitiveComponent Object Reference") (OtherBodyIndex :type Integer) (bFromSweep :type Boolean) (SweepResult :type "HitResult Structure (by ref)"))
  (if (== OtherActor (`GameplayStatics.GetPlayerPawn` 0))
    (`GameplayStatics.ApplyDamage` null 1.0)
    (`self.Fade&restart` :!label _label)))

(event `self.ReceiveTick`
  (params (DeltaSeconds :type "Float (single-precision)"))
  (goto _label :!via `execute2`))

(fn `UserConstructionScript`)