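; Level-exit trigger volume that advances the game once the player overlaps its box and every crystal in the level has been collected.
; A class search finding zero Bp_krysztal actors counts as complete; otherwise it only prints a debug string.
; Macros filter for the player pawn and quit the game on the last level.
; Otherwise it opens the entry following the current level's name in LevelList.
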(event `self.Box.OnComponentBeginOverlap`
  (params (OverlappedComponent :type "PrimitiveComponent Object Reference") (OtherActor :type "Actor Object Reference") (OtherComp :type "PrimitiveComponent Object Reference") (OtherBodyIndex :type Integer) (bFromSweep :type Boolean) (SweepResult :type "HitResult Structure (by ref)"))
  (`self.Is_player` OtherActor)
  (if (`self.Check_all_crystals`)
    (`self.Is_last_level`
      (:`return`
        (`self.Next_level`)))
    (else
      (`KismetSystemLibrary.PrintString` "Hello"))))

(fn `Check_all_crystals`
  (returns (ReturnValue :type Boolean))
  (bind _outactors (`GameplayStatics.GetAllActorsOfClass` "/Game/levels/klasy/actors/bp_krysztal.bp_krysztal_C"))
  (return (== (`KismetArrayLibrary.Array_Length` _outactors) 0)))

(fn `find current level name`
  (returns (ReturnValue :type Integer))
  (bind _returnvalue (`GameplayStatics.GetCurrentLevelName` true))
  (return (`KismetArrayLibrary.Array_Find` (`self.level_list`) (`KismetStringLibrary.Conv_StringToName` _returnvalue))))

(fn `Next_level`
  (`GameplayStatics.OpenLevel` (`|GetArrayItem` (`self.level_list`) (+ (`self.find current level name`) 1)) false))

(fn `UserConstructionScript`)